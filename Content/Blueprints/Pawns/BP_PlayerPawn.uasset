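; Player pawn moved by physics: axis inputs add torque to its mesh, scaled by a multiplier and applied as acceleration change, so mass is ignored.
; The camera fades in on BeginPlay; any damage runs a once-only macro that fades picture and audio out, then reopens the current level.
; A spring arm function sets camera distance, but its pitch rotation is disconnected and never runs.
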(event `self.ReceiveBeginPlay`
  (`PlayerCameraManager.StartCameraFade` :`self` (`GameplayStatics.GetPlayerCameraManager` 0) :`FromAlpha` 1.0 :`Duration` 3.0))

(event `InputAxis|Move Forward/Backwards`
  (params (AxisValue :type "Float (single-precision)"))
  (`PrimitiveComponent.AddTorqueInRadians` (`self.PlayerMesh`) (`KismetMathLibrary.MakeVector` 0.0 (* AxisValue (`self.TorqueMultiplier`) 5.0)) "None" true))

(event `InputAxis|Move Left/Right`
  (params (AxisValue :type "Float (single-precision)"))
  (`PrimitiveComponent.AddTorqueInRadians` (`self.PlayerMesh`) (`KismetMathLibrary.MakeVector` (* AxisValue (`self.TorqueMultiplier`) 5.0)) "None" true))

(event `self.ReceiveAnyDamage`
  (params (Damage :type "Float (single-precision)") (DamageType :type "DamageType Object Reference") (InstigatedBy :type "Controller Object Reference") (DamageCauser :type "Actor Object Reference"))
  (`self.Restart Level_Macro`))

(fn `Adjust Spring Arm_F`
  (params (Distance :type "Float (double-precision)") (Pitch :type "Float (double-precision)"))
  (set `SpringArmComponent.TargetArmLength` Distance (`self.SpringArm`)))

(fn `UserConstructionScript`)