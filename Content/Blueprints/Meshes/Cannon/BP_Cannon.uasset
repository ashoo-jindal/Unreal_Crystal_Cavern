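; BP_Cannon is a cannon that fires automatically and repeatedly from BeginPlay.
; Each cycle waits FireRate seconds, then spawns an actor at ArrowSpawnPoint's location and rotation, scaled by ProjectileScale.
; A backfire timeline then animates the barrel's local Y position for recoil, and its event track restarts the delay to keep the loop running.
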(event `self.ReceiveBeginPlay`
  (`KismetSystemLibrary.Delay` (`self.Fire Rate`) :!label _label)
  (`self.Spawn Projectile_F`)
  (bind (_direction _cannon_barrol_location) (`Timeline|Cannon_Backfire_TimeLine` :!via `PlayFromStart`)
    (:`Update`
      (`self.Move Cannon Barrel_F` _cannon_barrol_location))
    (:`Connon Fired`
      (goto _label))))

(fn `Move Cannon Barrel_F`
  (params (`Cannon Barrel Y Loc` :type "Float (double-precision)"))
  (`SceneComponent.K2_SetRelativeLocation` (`self.Cannon_Barrel`) (`KismetMathLibrary.MakeVector` 0.0 `Cannon Barrel Y Loc`) false false))

(fn `Spawn Projectile_F`
  (bind _arrow_spawn_point (`self.Arrow Spawn Point`))
  (`|SpawnActorFromClass` "/Game/Blueprints/Projectiles/BP_Projectile.BP_Projectile_C" (`KismetMathLibrary.MakeTransform` (`SceneComponent.K2_GetComponentLocation` _arrow_spawn_point) (`SceneComponent.K2_GetComponentRotation` _arrow_spawn_point) (`KismetMathLibrary.Conv_DoubleToVector` (`self.Projectile Scale`))) "Undefined" "OverrideRootScale" null null))

(fn `UserConstructionScript`)