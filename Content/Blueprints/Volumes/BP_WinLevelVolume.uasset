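; BP_WinLevelVolume is a trigger volume that completes the level when the player overlaps it and no BP_Crystal actors remain.
; It checks for remaining crystals with GetAllActorsOfClass on each player overlap.
; On completion it finds the current level's index in a LevelNames array, then opens the next level by name or quits the game on the last one.
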(event `self.ReceiveActorBeginOverlap`
  (params (OtherActor :type "Actor Object Reference"))
  (`/Game/Blueprints/Libraries/CC_MacroLibrary.IsPlayer_Macro` OtherActor
    (:`IsPlayer`
      (if (not (`self.Any Crystal Remaining_F`))
        (`self.Complete Level_F`)))))

(fn `Any Crystal Remaining_F`
  (returns (`Return Value` :type Boolean))
  (bind _outactors (`GameplayStatics.GetAllActorsOfClass` "/Game/Blueprints/Collectibles/BP_Crystal.BP_Crystal_C"))
  (return (> (`KismetArrayLibrary.Array_Length` _outactors) 0)))

(fn `Complete Level_F`
  (if (`self.Is Final Level_F`)
    (`KismetSystemLibrary.QuitGame` null "Quit")
    (else
      (`self.Load Next Level_F`))))

(fn `Get Current Level Index_F`
  (returns (`Return Value` :type Integer))
  (bind _returnvalue (`GameplayStatics.GetCurrentLevelName` true))
  (return (`KismetArrayLibrary.Array_Find` (`self.Level Names`) (`KismetStringLibrary.Conv_StringToName` _returnvalue))))

(fn `Get Next Level Name_F`
  (returns (`Return Value` :type Name))
  (return (`|GetArrayItem` (`self.Level Names`) (+ (`self.Get Current Level Index_F`) 1))))

(fn `Is Final Level_F`
  (returns (`Return Value` :type Boolean))
  (return (== (`KismetArrayLibrary.Array_LastIndex` (`self.Level Names`)) (`self.Get Current Level Index_F`))))

(fn `Load Next Level_F`
  (`GameplayStatics.OpenLevel` (`self.Get Next Level Name_F`)))

(fn `UserConstructionScript`)