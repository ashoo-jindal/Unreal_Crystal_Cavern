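; BP_Crystal is a collectible crystal that flies into the player and vanishes when the player overlaps it.
; On overlap it stores its location, scale and light intensity, then plays BlendTimeline.
; The timeline's separate tracks drive lerps that pull it toward the player's current position, shrink it to zero and fade its light.
; The actor destroys itself when the timeline finishes.
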(event `self.ReceiveActorBeginOverlap`
  (params (OtherActor :type "Actor Object Reference"))
  (`/Game/Blueprints/Libraries/CC_MacroLibrary.IsPlayer_Macro` OtherActor
    (:`IsPlayer`
      (`self.Store Starting Loc Values_F`)
      (bind (_direction _collection_progress _scale_progress _light_intensity) (`Timeline|BlendTimeline`)
        (:`Update`
          (`self.Move To Player_F` _collection_progress)
          (`self.Scale Crystal_F` _scale_progress)
          (`self.Adjust Light_F` _light_intensity))
        (:`Finished`
          (`self.K2_DestroyActor`))))))

(fn `Adjust Light_F`
  (params (Alpha :type "Float (double-precision)"))
  (`LightComponent.SetIntensity` (`self.CrystalLight`) (`KismetMathLibrary.Lerp` (`self.Start Light Intensity`) 0.0 Alpha)))

(fn `Move To Player_F`
  (params (Alpha :type "Float (double-precision)"))
  (`self.K2_SetActorLocation` (`KismetMathLibrary.VLerp` (`self.Lerp Start Location`) (`self.K2_GetActorLocation` (`GameplayStatics.GetPlayerPawn` 0)) Alpha)))

(fn `Scale Crystal_F`
  (params (Alpha :type "Float (double-precision)"))
  (`self.SetActorScale3D` (`KismetMathLibrary.VLerp` (`self.Start Scale`) (0.0 0.0 0.0) Alpha)))

(fn `Store Starting Loc Values_F`
  (set `self.Lerp Start Location` (`self.K2_GetActorLocation`))
  (set `self.Start Scale` (`self.GetActorScale3D`))
  (set `self.Start Light Intensity` (`LightComponentBase.Intensity` (`self.CrystalLight`))))

(fn `UserConstructionScript`)